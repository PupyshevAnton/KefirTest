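; BP_House is an interactable house actor that highlights itself and toggles the house interaction UI.
; The construction script copies the house mesh onto an outline mesh and fills its material slots with dynamic instances of an outline material.
; The Interact event shows or hides that outline and calls the matching show or hide function on the player controller cached at BeginPlay.
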(event Custom|SetOutline
  (Development|SetHiddeninGame (Variables|Default|GetHouseOutline) false false))

(event Custom|RemoveOutline
  (Development|SetHiddeninGame (Variables|Default|GetHouseOutline) true false))

(event EventBeginPlay
  (bind _asbp_player_controller (Utilities|Casting|CastToBP_PlayerController (Game|GetPlayerController 0)))
  (Variables|Default|SetBPPlayerController _asbp_player_controller))

(event EventInteract
  (params (bInteract :type Boolean))
  (bind _bpplayercontroller (Variables|Default|GetBPPlayerController))
  (if bInteract
    (CallFunction|SetOutline)
    (Default|ShowInteractHouse _bpplayercontroller)
    (else
      (CallFunction|RemoveOutline)
      (Default|HideInteractHouse _bpplayercontroller))))

(fn ConstructionScript
  (bind _houseoutline (Variables|Default|GetHouseOutline))
  (Components|StaticMesh|SetStaticMesh _houseoutline (Variables|/Script/Engine.StaticMeshComponent|GetStaticMesh (Variables|Default|GetHouseMesh)))
  (for (_ _array_index) (Rendering|Material|GetMaterials _houseoutline)
    (Rendering|Material|CreateDynamicMaterialInstance _houseoutline _array_index "/Game/KefirFarmTest/Materials/MI_InteractOutline.MI_InteractOutline" "None" :!class /Script/Engine.PrimitiveComponent)))