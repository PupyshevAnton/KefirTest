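; BP_CounterSell is an interactable sell counter that highlights itself and toggles the player's sell interaction UI.
; BeginPlay caches BP_PlayerController, and the Interact event uses its flag to show or hide both the outline and that UI.
; The construction script copies the counter's mesh onto CounterOutline and gives every material slot a dynamic instance of MI_InteractOutline, so the highlight is a toggled duplicate mesh.
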(event Custom|SetOutline
  (Development|SetHiddeninGame (Variables|Default|GetCounterOutline) false false))

(event Custom|RemoveOutline
  (Development|SetHiddeninGame (Variables|Default|GetCounterOutline) true false))

(event EventBeginPlay
  (bind _asbp_player_controller (Utilities|Casting|CastToBP_PlayerController (Game|GetPlayerController 0)))
  (Variables|Default|SetBPPlayerController _asbp_player_controller))

(event EventInteract
  (params (bInteract :type Boolean))
  (bind _bpplayercontroller (Variables|Default|GetBPPlayerController))
  (if bInteract
    (CallFunction|SetOutline)
    (Default|ShowInteractSell _bpplayercontroller)
    (else
      (CallFunction|RemoveOutline)
      (Default|HideInteractSell _bpplayercontroller))))

(fn ConstructionScript
  (bind _counteroutline (Variables|Default|GetCounterOutline))
  (Components|StaticMesh|SetStaticMesh _counteroutline (Variables|/Script/Engine.StaticMeshComponent|GetStaticMesh (Variables|Default|GetCounterMesh)))
  (for (_ _array_index) (Rendering|Material|GetMaterials _counteroutline)
    (Rendering|Material|CreateDynamicMaterialInstance _counteroutline _array_index "/Game/KefirFarmTest/Materials/MI_InteractOutline.MI_InteractOutline" "None" :!class /Script/Engine.PrimitiveComponent)))