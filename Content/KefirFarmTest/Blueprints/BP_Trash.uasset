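; BP_Trash is an interactable trash object in the farm game.
; Its Interact event shows or hides an outline mesh and tells the cached BP_PlayerController to show or hide the trash interaction, passing itself when shown.
; The construction script sets the mesh from the Trash variable, mirrors it onto the outline component and applies a dynamic outline material to every slot.
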(event Custom|SetOutline
  (Development|SetHiddeninGame (Variables|Default|GetTrashOutline) false false))

(event Custom|RemoveOutline
  (Development|SetHiddeninGame (Variables|Default|GetTrashOutline) true false))

(event EventBeginPlay
  (bind _asbp_player_controller (Utilities|Casting|CastToBP_PlayerController (Game|GetPlayerController 0)))
  (Variables|Default|SetBPPlayerController _asbp_player_controller))

(event EventInteract
  (params (bInteract :type Boolean))
  (bind _bpplayercontroller (Variables|Default|GetBPPlayerController))
  (if bInteract
    (CallFunction|SetOutline)
    (Default|ShowInteractTrash _bpplayercontroller self)
    (else
      (CallFunction|RemoveOutline)
      (Default|HideInteractTrash _bpplayercontroller))))

(fn ConstructionScript
  (bind _trashmesh (Variables|Default|GetTrashMesh))
  (bind _trashoutline (Variables|Default|GetTrashOutline))
  (Components|StaticMesh|SetStaticMesh _trashmesh (Variables|Default|GetTrash))
  (Components|StaticMesh|SetStaticMesh _trashoutline (Variables|/Script/Engine.StaticMeshComponent|GetStaticMesh _trashmesh))
  (for (_ _array_index) (Rendering|Material|GetMaterials _trashoutline)
    (Rendering|Material|CreateDynamicMaterialInstance _trashoutline _array_index "/Game/KefirFarmTest/Materials/MI_InteractOutline.MI_InteractOutline" "None" :!class /Script/Engine.PrimitiveComponent)))