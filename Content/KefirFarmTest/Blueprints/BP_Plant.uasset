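; BP_Plant is an interactable farm plant in a bed, with outline meshes for highlighting.
; Its Interact event toggles both outlines, shows or hides the plant prompt on BP_PlayerController, and sets or clears InteractPlantCode there.
; The construction script applies the Plant mesh, mirrors bed and plant meshes onto their outlines, and creates MI_InteractOutline dynamic materials, with plant setup nested inside the bed-material loop.
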(event Custom|SetOutline
  (Development|SetHiddeninGame (Variables|Default|GetBedOutline) false false)
  (Development|SetHiddeninGame (Variables|Default|GetPlantOutline) false false))

(event Custom|RemoveOutline
  (Development|SetHiddeninGame (Variables|Default|GetBedOutline) true false)
  (Development|SetHiddeninGame (Variables|Default|GetPlantOutline) true false))

(event Custom|SetInteractCode
  (params (PlayerController :type BP%20Player%20Controller%20Object%20Reference))
  (Variables|/Game/KefirFarmTest/BP_PlayerController.BP_PlayerController_C|SetInteractPlantCode PlayerController (Variables|Default|GetPlantCode)))

(event Custom|ClearInteractCode
  (params (PlayerController :type BP%20Player%20Controller%20Object%20Reference))
  (Variables|/Game/KefirFarmTest/BP_PlayerController.BP_PlayerController_C|SetInteractPlantCode PlayerController ""))

(event EventBeginPlay)

(event EventInteract
  (params (bInteract :type Boolean))
  (bind _asbp_player_controller (Utilities|Casting|CastToBP_PlayerController (Game|GetPlayerController 0)))
  (if bInteract
    (CallFunction|SetOutline)
    (Default|ShowInteractPlant _asbp_player_controller self)
    (CallFunction|SetInteractCode _asbp_player_controller)
    (else
      (CallFunction|RemoveOutline)
      (Default|HideInteractPlant _asbp_player_controller)
      (CallFunction|ClearInteractCode _asbp_player_controller))))

(fn ConstructionScript
  (bind _bedoutline (Variables|Default|GetBedOutline))
  (bind _plantoutline (Variables|Default|GetPlantOutline))
  (bind _plantmesh (Variables|Default|GetPlantMesh))
  (Components|StaticMesh|SetStaticMesh _bedoutline (Variables|/Script/Engine.StaticMeshComponent|GetStaticMesh (Variables|Default|GetBedMesh)))
  (for (_ _array_index) (Rendering|Material|GetMaterials _bedoutline)
    (Rendering|Material|CreateDynamicMaterialInstance _bedoutline _array_index "/Game/KefirFarmTest/Materials/MI_InteractOutline.MI_InteractOutline" "None" :!class /Script/Engine.PrimitiveComponent)
    (Components|StaticMesh|SetStaticMesh _plantmesh (Variables|Default|GetPlant))
    (Components|StaticMesh|SetStaticMesh _plantoutline (Variables|/Script/Engine.StaticMeshComponent|GetStaticMesh _plantmesh))
    (for (_ _array_index_2) (Rendering|Material|GetMaterials _plantoutline)
      (Rendering|Material|CreateDynamicMaterialInstance _plantoutline _array_index_2 "/Game/KefirFarmTest/Materials/MI_InteractOutline.MI_InteractOutline" "None" :!class /Script/Engine.PrimitiveComponent))))